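; Shootable LED spotlight prop that can be switched on and off until it is destroyed.
; A GunFireHitTarget hit removes the glass and spotlight, spawns a physics-simulated destructible component with the destroyed cover material, and plays a glass sound.
; TurnMeOn and TurnMeOff set spotlight intensity and swap the glass material, and a Destroyed flag disables both, along with further hit reactions.
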(event `self.ReceiveBeginPlay`
  (add `/Game/Playground/BPs/GunFireHitTarget.Hit` (`self.GunFireHitTarget`) (delegate `GotShot`)))

(event `GotShot`
  (params (LocationLS :type "Vector Structure") (LocationWS :type "Vector Structure") (Normal :type "Vector Structure"))
  (if (not (`self.Destroyed`))
    (`ActorComponent.K2_DestroyComponent` (`self.Light_glass`))
    (`ActorComponent.K2_DestroyComponent` (`self.SpotLight1`))
    (bind _returnvalue (`AddComponent|NODE_AddDestructibleComponent-0`))
    (`PrimitiveComponent.SetSimulatePhysics` _returnvalue true)
    (`PrimitiveComponent.SetMaterial` _returnvalue 0 "/Game/Playground/Environment/LED/LightCoverDestroyed.LightCoverDestroyed")
    (set `self.Destroyed` true)
    (`GameplayStatics.PlaySoundAtLocation` "/Game/Playground/Sounds/glass2.glass2" (`self.K2_GetActorLocation`))))

(fn `TurnMeOff`
  (if (not (`self.Destroyed`))
    (`LightComponent.SetIntensity` (`self.SpotLight1`) 0.0)
    (`PrimitiveComponent.SetMaterial` (`self.Light_glass`) 0 "/Game/Playground/Environment/LED/LightCoverDestroyed.LightCoverDestroyed")))

(fn `TurnMeOn`
  (if (not (`self.Destroyed`))
    (`LightComponent.SetIntensity` (`self.SpotLight1`) 5000.0)
    (`PrimitiveComponent.SetMaterial` (`self.Light_glass`) 0 "/Game/Playground/Environment/LED/LightCover.LightCover")))

(fn `UserConstructionScript`)