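; Shooting target that shows bullet marks, scores hits by closeness to its center and slides away along world Y after ten hits.
; GunFireHitTarget feeds hits into a drawer material that paints each local position onto a per-instance render target, displayed by the plane's dynamic material.
; The first nine hits add to a score shown on TextRender, which ResetScore zeroes.
; Tick continuously moves the actor toward DesiredY.
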(event `self.ReceiveBeginPlay`
  (add `/Game/Playground/BPs/GunFireHitTarget.Hit` (`self.GunFireHitTarget`) (delegate `Hit`))
  ;[1 1 1] Create dynamic material for bullet decals
  (bind _returnvalue (`KismetRenderingLibrary.CreateRenderTarget2D` 1024 1024))
  (bind _output_get (set `self.RenderTarget` _returnvalue))
  (`KismetRenderingLibrary.ClearRenderTarget2D` _output_get (struct :`R` 1.0 :`G` 1.0 :`B` 1.0 :`A` 1.0))
  (bind _returnvalue_2 (`KismetMaterialLibrary.CreateDynamicMaterialInstance` "/Game/Playground/Environment/target/TargetMatDynamic.TargetMatDynamic"))
  (bind _output_get_2 (set `self.TargetMat` _returnvalue_2))
  (`PrimitiveComponent.SetMaterial` (`self.Plane`) 0 _output_get_2)
  (`MaterialInstanceDynamic.SetTextureParameterValue` _output_get_2 "RenderTarget" (`self.RenderTarget`))
  (bind _returnvalue_3 (`KismetMaterialLibrary.CreateDynamicMaterialInstance` "/Game/Playground/Environment/target/bullet_drawer.bullet_drawer"))
  (set `self.DrawerMat` _returnvalue_3))

(event `Hit`
  (params (LocationLS :type "Vector Structure") (LocationWS :type "Vector Structure") (Normal :type "Vector Structure"))
  (bind _drawermat (`self.DrawerMat`))
  (`/Engine/EditorBlueprintResources/StandardMacros.IncrementInt` (`self.NumHits`)
    (:`  `
      ;[1 1 1] All transparent decal
      (`MaterialInstanceDynamic.SetVectorParameterValue` _drawermat "Position" (`KismetMathLibrary.Conv_VectorToLinearColor` (+ (/ LocationLS 100.0) 0.5)))
      (`KismetRenderingLibrary.DrawMaterialToRenderTarget` (`self.RenderTarget`) _drawermat)
      (if (>= (`self.NumHits`) 10)
        (set `self.DesiredY` -550.0)
        (else
          ;[1 1 1] Calculate Score
          (bind _output_get (set `self.Score` (+ (`KismetMathLibrary.FTrunc` (* (`KismetMathLibrary.FClamp` (- 1.0 (/ (`KismetMathLibrary.VSize` LocationLS) 40.0))) 100.0)) (`self.Score`))))
          (`TextRenderComponent.K2_SetText` (`self.TextRender`) (`KismetTextLibrary.Conv_StringToText` (`KismetStringLibrary.Concat_StrStr` "Score: " (`KismetStringLibrary.Conv_IntToString` _output_get)))))))))

(event `self.ReceiveTick`
  (params (DeltaSeconds :type "Float (single-precision)"))
  (bind _y (.y (`self.K2_GetActorLocation`)))
  (`self.K2_SetActorLocation` (`KismetMathLibrary.MakeVector` (.x (`self.K2_GetActorLocation`)) (+ _y (* (* DeltaSeconds 100.0) (`KismetMathLibrary.FClamp` (- (`self.DesiredY`) _y) -1.0))) (.z (`self.K2_GetActorLocation`)))))

(fn `ResetScore`
  (set `self.Score` 0)
  (`TextRenderComponent.K2_SetText` (`self.TextRender`) "Score: 0"))

(fn `UserConstructionScript`)